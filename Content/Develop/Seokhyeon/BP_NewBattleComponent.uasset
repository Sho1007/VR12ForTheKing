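; BP_NewBattleComponent is a battle component that overrides Attack and Action, with Action intended for enemy AI.
; Action picks a random ActionArray entry from DT_Action and, for Attack types, sets ActionTarget to a random character from MyGameModeBase's CharacterArray, without calling Attack.
; Attack calls its parent, then succeeds only if the target's faction differs.
; Beyond the parent calls, results are only debug prints and return values.
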(event EventBeginPlay)

(event EventTick
  (params (DeltaSeconds :type Float%20%28single-precision%29)))

(fn Attack
  (bind _actiontarget (Variables|Default|GetActionTarget))
  (|CallParentFunction)
  (if (Utilities|Enum|NotEqual(Enum) (Variables|/Script/VR12ForTheKing.BattleComponent|GetFactionType (Variables|/Script/VR12ForTheKing.MyCharacter|GetBattleComponent _actiontarget)) (Variables|Default|GetFactionType))
    (Development|PrintString (Utilities|String|Append "Attack To" (Utilities|GetDisplayName _actiontarget)))
    (return true)
    (else
      (Development|PrintString "Can not Attack Your Faction")
      (return false))))

(fn Action
  ;[1 1 1] 무조건 Enemy (AI) 에서 실행
  (|CallParentFunction)
  (Development|PrintString "Hello")
  (bind _returnvalue (Utilities|GetDataTableRow "/Game/Develop/Seokhyeon/Data/DT_Action.DT_Action" (.OutItem (Utilities|Array|Random (Variables|Default|GetActionArray))))
    (:then
      (switch Utilities|FlowControl|Switch|SwitchonEActionType (.actiontype _returnvalue)
        (:Attack
          (bind _asmy_game_mode_base (Utilities|Casting|CastToMyGameModeBase (Game|GetGameMode)))
          (Variables|Default|SetActionTarget (.OutItem (Utilities|Array|Random (Variables|/Script/VR12ForTheKing.MyGameModeBase|GetCharacterArray _asmy_game_mode_base))))
          (Development|PrintString (Utilities|String|ToString(Text) (.name _returnvalue)))
          (return true))))
    (:RowNotFound
      (Development|PrintString "Cannot Found Action")
      (return false))))