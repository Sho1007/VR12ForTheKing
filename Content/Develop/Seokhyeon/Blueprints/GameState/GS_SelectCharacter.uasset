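; GameState for the character selection screen, tracking which player controller occupies each slot in CharacterDataArray.
; SetPlayer writes a controller into the requested slot only if that slot is empty.
; The array's RepNotify fetches the local HUD_SelectCharacter and loops over the entries, but the loop body is unfinished, so it only prints debug text and caches the HUD.
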(event EventBeginPlay)

(event EventTick
  (params (DeltaSeconds :type Float%20%28single-precision%29)))

(fn ConstructionScript)

(fn OnRepCharacterDataArray
  (Development|PrintString "OnRep")
  (bind _ashud_select_character (Utilities|Casting|CastToHUD_SelectCharacter (HUD|GetHUD (Game|GetPlayerController 0))))
  (LocalVariables|SetSelectHUD _ashud_select_character)
  (for _array_element (Variables|Default|GetCharacterDataArray)
    (if (!= _array_element 0)
      _)))

(fn SetPlayer
  (params (SlotIndex :type Integer) (PlayerController :type Player%20Controller%20Object%20Reference))
  (Development|PrintString "SetPlayer")
  (Utilities|IsValid (Utilities|Array|Get(acopy) (Variables|Default|GetCharacterDataArray) SlotIndex)
    (:Is%20Valid
      (Development|PrintString "Slot is not empty")
      (return))
    (:Is%20Not%20Valid
      (Utilities|Array|SetArrayElem (Variables|Default|GetCharacterDataArray) SlotIndex PlayerController))))