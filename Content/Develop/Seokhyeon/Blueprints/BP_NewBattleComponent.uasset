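; Battle component subclass that overrides Attack and BattleAction, apparently a work-in-progress version of a combat action system.
; BattleAction runs the parent logic, then randomly draws from ActionArray to call Attack on NormalAttack, otherwise draws again and only prints on WeakHeal.
; Attack just defers to the parent; its faction-based targeting and debug-print logic is disconnected and never runs.
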(event EventBeginPlay)

(event EventTick
  (params (DeltaSeconds :type Float%20%28single-precision%29)))

(fn Attack
  (|CallParentFunction))

(fn BattleAction
  (bind _actionarray (Variables|Default|GetActionArray))
  (bind _outitem (Utilities|Array|Random _actionarray))
  (|CallParentFunction)
  (Development|PrintString "Called Battle Action")
  (if (== _outitem "NormalAttack")
    (CallFunction|Attack)
    (elif (== _outitem "WeakHeal")
      (Development|PrintString "WeakHeal"))))