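; BP_Grid is a tile grid actor that draws its lines procedurally and can highlight a selected tile.
; The construction script uses CreateLine quads to build the line mesh and a hidden, tile-sized selection mesh, each with a dynamic M_Grid material for color and opacity.
; LocationToTile and TileToGridLocation convert between world positions and row/column, checked by TileValid.
; SetSelectedTile moves the selection mesh to a valid tile or hides it.
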(event EventBeginPlay)

(fn ConstructionScript
  (bind _tilesize (Variables|Constents|GetTileSize))
  (bind _returnvalue (/ _tilesize 2.0))
  ;[1 1 1] 라인
  (bind _materialistance (Private|CreateMaterialInstance (Variables|Constents|GetLineColor) (Variables|Constents|GetLineOpacity)))
  (LocalVariables|SetLinesMaterialInstance _materialistance)
  ;[1 1 1] 사각형
  (bind _materialistance_2 (Private|CreateMaterialInstance (Variables|Constents|GetSelectionColor) (Variables|Constents|GetSelectionOpacity)))
  (LocalVariables|SetSelectionMaterialInstance _materialistance_2)
  (Utilities|FlowControl|Sequence
    (:then_0
      ;[1 1 1] Create horizontal line geometry(수평선 기하학 만들기)
      (for _index (range 0 (Variables|Constents|GetNumRows))
        (LocalVariables|SetLineStart (* _index (Variables|Constents|GetTileSize)))
        (LocalVariables|SetLineEnd (Private|GridWidth))
        (Private|CreateLine (Math|Vector|MakeVector (LocalVariables|GetLineStart) 0.0 0.0) (Math|Vector|MakeVector (LocalVariables|GetLineStart) (LocalVariables|GetLineEnd) 0.0) (Variables|Constents|GetLineThickness) (LocalVariables|GetLineVertices) (LocalVariables|GetLineTriangles))))
    (:then_1
      ;[1 1 1] Create vertical line geometry(수직선 기하학 만들기)
      (for _index_2 (range 0 (Variables|Constents|GetNumColums))
        (LocalVariables|SetLineStart (* _index_2 (Variables|Constents|GetTileSize)))
        (LocalVariables|SetLineEnd (Private|GridHeigh))
        (Private|CreateLine (Math|Vector|MakeVector 0.0 (LocalVariables|GetLineStart) 0.0) (Math|Vector|MakeVector (LocalVariables|GetLineEnd) (LocalVariables|GetLineStart) 0.0) (Variables|Constents|GetLineThickness) (LocalVariables|GetLineVertices) (LocalVariables|GetLineTriangles))))
    (:then_2
      ;[1 1 1 1 15] create the procedural mesh for the line(선에 대한 절차적 메시 생성)
      (Class|ProceduralMeshComponent|CreateMeshSectionLinearColor (Variables|Default|GetLinesProceduralMesh) 0 (LocalVariables|GetLineVertices) (LocalVariables|GetLineTriangles) 0 0 0 0 0 0 0 false false)
      (Rendering|Material|SetMaterial (Variables|Default|GetLinesProceduralMesh) 0 (LocalVariables|GetLinesMaterialInstance)))
    (:then_3
      ;[1 1 1] 선택 구역(네모) 및 색 설정
      (Private|CreateLine (Math|Vector|MakeVector 0.0 _returnvalue 0.0) (Math|Vector|MakeVector _tilesize _returnvalue 0.0) (Variables|Constents|GetTileSize) (LocalVariables|GetSelectionVertices) (LocalVariables|GetSelectionTriangles))
      ;;[1 1 1] 가시성
      (Rendering|SetVisibility (Variables|Default|GetSelectionProceduralMesh) false false)
      (Class|ProceduralMeshComponent|CreateMeshSectionLinearColor (Variables|Default|GetSelectionProceduralMesh) 0 (LocalVariables|GetSelectionVertices) (LocalVariables|GetSelectionTriangles) 0 0 0 0 0 0 0 false false)
      (Rendering|Material|SetMaterial (Variables|Default|GetSelectionProceduralMesh) 0 (LocalVariables|GetSelectionMaterialInstance)))))

(fn CreateLine
  (params (Start :type Vector) (End :type Vector) (Thinkness :type Float%20%28double-precision%29) (Vertices :type Array%20of%20Vectors) (Triangles :type Array%20of%20Integers))
  (bind _returnvalue (Utilities|Array|Length (Variables|Default|GetVertices)))
  (Utilities|FlowControl|Sequence
    (:then_0
      ;[1 1 1] 선 두께의 반
      (LocalVariables|SetHalfThickness (/ (Variables|Default|GetThinkness) 2.0))
      ;[1 1 1] 두께가 적용되어야하는 방향
      (LocalVariables|SetThicknessDirection (Math|Vector|CrossProduct (Math|Vector|Normalize (- (Variables|Default|GetEnd) (Variables|Default|GetStart))) "0.000000,0.000000,1.000000")))
    (:then_1
      (Utilities|Array|AppendArray (Variables|Default|GetTriangles) (Utilities|Array|MakeArray (+ _returnvalue 2) (+ _returnvalue 1) (+ _returnvalue 0) (+ _returnvalue 2) (+ _returnvalue 3) (+ _returnvalue 1)))
      ;[1 1 1] 꼭지점을 추가하는 역할
      (Utilities|Array|AppendArray (Variables|Default|GetVertices) (Utilities|Array|MakeArray (+ Start (* (LocalVariables|GetThicknessDirection) (LocalVariables|GetHalfThickness))) (+ (Variables|Default|GetEnd) (* (LocalVariables|GetThicknessDirection) (LocalVariables|GetHalfThickness))) (- Start (* (LocalVariables|GetThicknessDirection) (LocalVariables|GetHalfThickness))) (- (Variables|Default|GetEnd) (* (LocalVariables|GetThicknessDirection) (LocalVariables|GetHalfThickness))))))))

(fn GridWidth
  (return (* (Variables|Constents|GetNumColums) (Variables|Constents|GetTileSize))))

(fn GridHeigh
  (return (* (Variables|Constents|GetNumRows) (Variables|Constents|GetTileSize))))

(fn CreateMaterialInstance
  (params (Color :type Linear%20Color%20Structure) (Opacity :type Float%20%28double-precision%29))
  (bind _returnvalue (Rendering|Material|CreateDynamicMaterialInstance "/Game/Develop/CH/Blueprints/M_Grid.M_Grid" "None" "None" :!class /Script/Engine.KismetMaterialLibrary))
  (Rendering|Material|SetVectorParameterValue _returnvalue "Color" Color :!class /Script/Engine.MaterialInstanceDynamic)
  (Rendering|Material|SetScalarParameterValue _returnvalue "Opacity" Opacity :!class /Script/Engine.MaterialInstanceDynamic)
  (return _returnvalue))

(fn LocationtoTile
  (params (Location :type Vector))
  (bind _returnvalue (Transformation|GetActorLocation))
  (bind _returnvalue_2 (Private|GridHeigh))
  (bind _returnvalue_3 (Transformation|GetActorLocation))
  (bind _returnvalue_4 (Private|GridWidth))
  (bind _numcolums (Variables|Constents|GetNumColums))
  (bind _numrows (Variables|Constents|GetNumRows))
  (bind _returnvalue_5 (- (.y (Variables|Default|GetLocation)) (.y _returnvalue)))
  (bind _returnvalue_6 (- (.x (Variables|Default|GetLocation)) (.x _returnvalue_3)))
  (bind _returnvalue_7 (/ _returnvalue_5 _returnvalue_2))
  (bind _returnvalue_8 (/ _returnvalue_6 _returnvalue_4))
  (bind _returnvalue_9 (* _numcolums _returnvalue_7))
  (bind _returnvalue_10 (* _numrows _returnvalue_8))
  (bind _returnvalue_11 (Math|Float|Floor _returnvalue_9))
  (bind _returnvalue_12 (Math|Float|Floor _returnvalue_10))
  (bind _valid (Utilities|TileValid _returnvalue_12 _returnvalue_11))
  (return _valid _returnvalue_12 _returnvalue_11))

(fn TiletoGridLocation
  (params (Row :type Integer) (Column :type Integer) (Center :type Boolean))
  (bind _valid (Utilities|TileValid Row Column)))

(fn SetSelectedTile
  (params (Row :type Integer) (Column :type Integer))
  (bind (_valid _gridlocation) (CallFunction|TiletoGridLocation Row Column false))
  (if _valid
    (Rendering|SetVisibility (Variables|Default|GetSelectionProceduralMesh) true false)
    (Transformation|SetWorldLocation (Variables|Default|GetSelectionProceduralMesh) (Math|Vector|MakeVector (.X (Math|Vector2D|BreakVector2D _gridlocation)) (.Y (Math|Vector2D|BreakVector2D _gridlocation)) (.z (Transformation|GetActorLocation))) false false)
    (else
      (Rendering|SetVisibility (Variables|Default|GetSelectionProceduralMesh) false false))))