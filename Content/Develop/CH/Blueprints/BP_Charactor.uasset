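; Character Blueprint apparently meant to drive cursor-based tile selection on a grid.
; Tick calls UpdateCursorPosition when no head-mounted display is active, but that function's entry is unwired, so it does nothing.
; Its disconnected logic traces under the cursor, aligns the 타깃 component to the hit surface, and selects the matching Grid tile, or clears selection on a miss.
; The game mode cast supplying the Grid has no target class.
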(event EventTick
  (params (DeltaSeconds :type Float%20%28single-precision%29))
  (if (not (Class|HeadMountedDisplayFunctionLibrary|IsHeadMountedDisplayEnabled))
    (CallFunction|UpdateCursorPosition)))

(fn ConstructionScript)

(fn UpdateCursorPosition)