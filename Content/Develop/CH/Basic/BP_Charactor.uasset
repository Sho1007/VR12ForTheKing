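; BP_Charactor is a player character Blueprint that drives cursor-based tile selection on a grid.
; Each tick without HMD tracking, it traces under the mouse on the Visibility channel and moves the 타깃 (target) component to the hit, oriented to the surface normal.
; It converts the hit to a tile and selects it on the grid from BP_GM, or passes -1 indices when nothing is hit.
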(event EventTick
  (params (DeltaSeconds :type Float%20%28single-precision%29))
  (if (not (Class|HeadMountedDisplayFunctionLibrary|IsHeadMountedDisplayEnabled))
    (CallFunction|UpdateCursorPosition)))

(fn ConstructionScript)

(fn UpdateCursorPosition
  (bind _returnvalue (Game|GetPlayerController 0))
  (bind (_hitresult _returnvalue_2) (Game|Player|GetHitResultUnderCursorbyChannel _returnvalue "TraceTypeQuery1" true))
  (bind (_bblockinghit _binitialoverlap _time _distance _location _impactpoint _normal _impactnormal) (Collision|BreakHitResult _hitresult))
  (bind _asbp_gm (Utilities|Casting|CastToBP_GM (Game|GetGameMode)))
  (LocalVariables|SetGrid (Default|GetGrid _asbp_gm))
  (if _returnvalue_2
    (bind _output_get (LocalVariables|SetHitLocation _location))
    (Transformation|SetWorldLocationAndRotation (Variables|Default|Get타깃) _output_get (Math|Rotator|MakeRotationfromAxes _impactnormal "0, 0, 0" "0, 0, 0") false false)
    (bind (_valid _row _column) (Default|LocationtoTile (LocalVariables|GetGrid) (LocalVariables|GetHitLocation)))
    (Default|SetSelectedTile (LocalVariables|GetGrid) _row _column)
    (else
      (Default|SetSelectedTile (LocalVariables|GetGrid) -1 -1))))