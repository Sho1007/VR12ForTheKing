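; Quest giver component that attaches to NPCs and offers a quest or shows its rewards on interaction.
; InteractWith queries the player's QuestLogComponent, opening the quest details widget if the quest is not active, or the rewards widget if its quest actor is completed.
; Both widgets receive data table rows keyed by QuestData.RowName, though rewards always read DT_TestQuestData rather than QuestData's table.
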(event EventBeginPlay)

(event EventTick
  (params (DeltaSeconds :type Float%20%28single-precision%29)))

(fn DisplayQuest
  (bind _questdata (Variables|Default|GetQuestData))
  ;[1 1 1] 퀘스트 세부정보 출력
  (bind _returnvalue (Utilities|GetDataTableRow (.datatable _questdata) (.rowname _questdata))
    (:then
      (bind _returnvalue_2 (UserInterface|CreateWidget "/Game/Develop/CH/QuestTutorial/QuestSystem/UI/Wg_QuestGiver.Wg_QuestGiver_C" 0 _returnvalue (.rowname _questdata)))
      (UserInterface|Viewport|AddtoViewport _returnvalue_2 0))))

(fn DisplayRewards
  (bind _questdata (Variables|Default|GetQuestData))
  ;[1 1 1] 퀘스트 보상 화면
  (bind _returnvalue (Utilities|GetDataTableRow "/Game/Develop/CH/QuestTutorial/QuestSystem/DT_TestQuestData.DT_TestQuestData" (.rowname _questdata))
    (:then
      (bind _returnvalue_2 (UserInterface|CreateWidget "/Game/Develop/CH/QuestTutorial/QuestSystem/UI/Wg_QuestRewards.Wg_QuestRewards_C" 0 _returnvalue (.rowname _questdata)))
      (UserInterface|Viewport|AddtoViewport _returnvalue_2 0))))

(fn Interactwith
  (bind _returnvalue (Components|GetOwner))
  (bind _returnvalue_2 (Utilities|GetDisplayName _returnvalue))
  ;[1 1 1] 모든 NPC에 부착할 수 있는 구성 요소
  (if (not (Default|QueryActiveQuest (Variables|/Game/Develop/CH/QuestTutorial/FirstPerson/BP_FirstPersonCharacter.BP_FirstPersonCharacter_C|GetQuestLogComponent (CallFunction|GetMyPlayerCharacter)) (.rowname (Variables|Default|GetQuestData))))
    (CallFunction|DisplayQuest)
    (return _returnvalue_2)
    (else
      ;;[1 1 1] 이미 완료되었는지 확인
      (bind _array_element (Default|GetQuestActor (Variables|/Game/Develop/CH/QuestTutorial/FirstPerson/BP_FirstPersonCharacter.BP_FirstPersonCharacter_C|GetQuestLogComponent (CallFunction|GetMyPlayerCharacter)) (.rowname (Variables|Default|GetQuestData))))
      (if (Variables|/Game/Develop/CH/QuestTutorial/Blueprints/BP_QuestBase.BP_QuestBase_C|GetIsCompleted _array_element)
        (CallFunction|DisplayRewards)
        (return _returnvalue_2)))))