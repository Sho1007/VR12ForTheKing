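; Inventory component for a quest tutorial that stores item quantities in a Content map.
; AddToInventory adds the given quantity to the stored count, then reports the item as an objective ID, with the added quantity, through player 0's BP_FirstPersonCharacter to drive quest objectives.
; QueryInventory returns the stored count for an item; BeginPlay and Tick are unused.
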(event EventBeginPlay)

(event EventTick
  (params (DeltaSeconds :type Float%20%28single-precision%29)))

(fn AddtoInventory
  (params (Item :type Name) (Quantitiy :type Integer))
  ;[1 1 1] 인벤토리에 항목을 추가할 때 완료한 목표를 호출하려고 함
  (Utilities|Map|Add (Variables|Default|GetContent) Item (+ Quantitiy (.Value (Utilities|Map|Find (Variables|Default|GetContent) Item))))
  (bind _asbp_first_person_character (Utilities|Casting|CastToBP_FirstPersonCharacter (Game|GetPlayerCharacter 0)))
  (Default|CallOnObjectiveIDCalled _asbp_first_person_character (Utilities|String|ToString(Name) Item) Quantitiy))

(fn QueryInventory
  (params (Item :type Name))
  (return (.Value (Utilities|Map|Find (Variables|Default|GetContent) Item))))