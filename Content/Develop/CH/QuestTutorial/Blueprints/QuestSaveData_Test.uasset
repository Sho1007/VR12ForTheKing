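; Quest save data container, apparently a test version, that stores and restores a quest log's state.
; SaveQuestLog copies the active and completed quest lists, while SaveQuestDetails stores each quest's stage and objective progress in a map keyed by quest ID.
; LoadQuests re-adds each active quest through the QuestLogComponent, restores its stage and progress from that map, then assigns both saved lists back to the component.
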(fn SaveQuestDetails
  (params (Quest :type BP%20Quest%20Base%20Object%20Reference))
  ;[1 1 1] 퀘스트 세부정보 저장
  (Utilities|Map|Add (Variables|Default|GetQuestProgress) (Variables|/Game/Develop/CH/QuestTutorial/Blueprints/BP_QuestBase.BP_QuestBase_C|GetQuestID_Test Quest) (Utilities|Struct|MakeS_QuestSaveData (Variables|/Game/Develop/CH/QuestTutorial/Blueprints/BP_QuestBase.BP_QuestBase_C|GetCurrentObjectiveProgress Quest) (Variables|/Game/Develop/CH/QuestTutorial/Blueprints/BP_QuestBase.BP_QuestBase_C|GetCurrentStage Quest))))

(fn LoadQuests
  (params (QuestLogComponent :type Quest%20Log%20Component%20Object%20Reference))
  (for _array_element (Variables|Default|GetCurrentActiveQuests)
    (bind _returnvalue (Default|AddNewQuest QuestLogComponent _array_element))
    (Variables|/Game/Develop/CH/QuestTutorial/Blueprints/BP_QuestBase.BP_QuestBase_C|SetCurrentStage _returnvalue (.CurrentStage (Utilities|Struct|BreakS_QuestSaveData (.Value (Utilities|Map|Find (Variables|Default|GetQuestProgress) _array_element)))))
    (Variables|/Game/Develop/CH/QuestTutorial/Blueprints/BP_QuestBase.BP_QuestBase_C|SetCurrentObjectiveProgress _returnvalue (.Progress (Utilities|Struct|BreakS_QuestSaveData (.Value (Utilities|Map|Find (Variables|Default|GetQuestProgress) _array_element))))))
  (Variables|/Game/Develop/CH/QuestTutorial/Blueprints/QuestLogComponent.QuestLogComponent_C|SetCurrentActiveQuests QuestLogComponent (Variables|Default|GetCurrentActiveQuests))
  (Variables|/Game/Develop/CH/QuestTutorial/Blueprints/QuestLogComponent.QuestLogComponent_C|SetCompletedQuests QuestLogComponent (Variables|Default|GetCompletedQuests)))

(fn SaveQuestLog
  (params (QuestLog :type Quest%20Log%20Component%20Object%20Reference))
  (Variables|Default|SetCurrentActiveQuests (Variables|/Game/Develop/CH/QuestTutorial/Blueprints/QuestLogComponent.QuestLogComponent_C|GetCurrentActiveQuests QuestLog))
  (Variables|Default|SetCompletedQuests (Variables|/Game/Develop/CH/QuestTutorial/Blueprints/QuestLogComponent.QuestLogComponent_C|GetCompletedQuests QuestLog)))