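; BP_QuestBase tracks one quest's progress through the objectives of its current stage.
; On BeginPlay it loads the stage from DT_TestQuestData into an ID-to-count map, binds to the player's objective-ID event, and credits matching inventory items for one objective type.
; Heard events adjust counts in either direction, adding only below the required quantity.
; Reaching a quantity shows a notification widget and re-evaluates IsCompleted across all objectives.
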(event EventBeginPlay
  (CallFunction|GetQuestDetails)
  (EventDispatchers|BindEventtoOnObjectiveIDCalled (CallFunction|GetMyPlayerCharacter) (EventDispatchers|CreateEvent :!event OnObjectiveIDHeard))
  ;[1 1 1] 인벤토리에 이미 퀘스트 아이템이 있는지 확인
  (for _array_element (Utilities|Struct|BreakS_StageDetails (Variables|Default|GetCurrentStageDetails))
    (if (Utilities|Enum|Equal(Enum) (.Type (Utilities|Struct|BreakS_ObjectiveDetails _array_element)) "NewEnumerator3")
      (bind _value (Default|QueryInventory (Variables|/Game/Develop/CH/QuestTutorial/FirstPerson/BP_FirstPersonCharacter.BP_FirstPersonCharacter_C|GetInventoryComponent (CallFunction|GetMyPlayerCharacter)) (Utilities|String|StringToName (.ObjectiveID (Utilities|Struct|BreakS_ObjectiveDetails _array_element)))))
      (CallFunction|OnObjectiveIDHeard (.ObjectiveID (Utilities|Struct|BreakS_ObjectiveDetails _array_element)) _value)))
  (bind _return (CallFunction|AreObjectivesComplete))
  (Variables|Default|SetIsCompleted _return))

(fn ConstructionScript)

(fn OnObjectiveIDHeard
  (params (ObjectiveID :type String) (Value :type Integer))
  (bind _currentobjectiveprogress (Variables|Default|GetCurrentObjectiveProgress))
  (bind (_value _returnvalue) (Utilities|Map|Find _currentobjectiveprogress ObjectiveID))
  (if (> (Class|KismetMathLibrary|SignOfInteger Value) 0)
    ;[1 1 1] 목표 진행상황 확인 후 일치하는 항목이 있는지 확인
    (if _returnvalue
      (if (< _value (Utilities|Struct|BreakS_ObjectiveDetails (CallFunction|GetObjectiveDatabyID ObjectiveID)))
        (Utilities|Map|Add (Variables|Default|GetCurrentObjectiveProgress) ObjectiveID (+ _value Value))
        (CallFunction|IsObjectiveComplete ObjectiveID)
        (return))
      (else
        (return)))
    (else
      ;[1 1 1] 목표 수의 값을 줄이는 경우에 변화되는 값을 확인
      (Utilities|Map|Add (Variables|Default|GetCurrentObjectiveProgress) ObjectiveID (+ (.Value (Utilities|Map|Find (Variables|Default|GetCurrentObjectiveProgress) ObjectiveID)) Value))
      (return))))

(fn GetQuestDetails
  ;[1 1 1] 요청 데이타 가져오고, 세부사항 처리
  (bind _returnvalue (Utilities|GetDataTableRow "/Game/Develop/CH/QuestTutorial/QuestSystem/DT_TestQuestData.DT_TestQuestData" (Variables|Default|GetQuestID_Test))
    (:then
      (bind _output_get (Variables|Default|SetQuestDetails _returnvalue))
      (bind _output_get_2 (Variables|Default|SetCurrentStageDetails (Utilities|Array|Get(acopy) (Utilities|Struct|BreakS_QuestDetails _output_get) (Variables|Default|GetCurrentStage))))
      ;[1 1 1] 진행할 개체 삭제
      (Utilities|Map|Clear (Variables|Default|GetCurrentObjectiveProgress))
      (for _array_element (Utilities|Struct|BreakS_StageDetails _output_get_2)
        ;[1 1 1] 객관적인 아이디어 다시 추가
        (Utilities|Map|Add (Variables|Default|GetCurrentObjectiveProgress) (.ObjectiveID (Utilities|Struct|BreakS_ObjectiveDetails _array_element)) 0)))))

(fn GetObjectiveDatabyID
  (params (ObjectiveID :type String))
  ;[1 1 1] 객관적인 데이타를 얻고 있는지
  (for _array_element (.Objectives (Utilities|Struct|BreakS_StageDetails (Variables|Default|GetCurrentStageDetails)))
    (if (Utilities|Enum|Equal(Enum) (Utilities|Struct|BreakS_ObjectiveDetails _array_element) ObjectiveID)
      (return _array_element))))

(fn IsObjectiveComplete
  (params (ObjectiveID :type String))
  (bind _array_element (CallFunction|GetObjectiveDatabyID ObjectiveID))
  (bind (_description _quantiy) (Utilities|Struct|BreakS_ObjectiveDetails _array_element))
  ;[1 1 1] 목표가 완료되었는지 확인 가능
  (if (>= (.Value (Utilities|Map|Find (Variables|Default|GetCurrentObjectiveProgress) ObjectiveID)) _quantiy)
    (bind _returnvalue (UserInterface|CreateWidget "/Game/Develop/CH/QuestTutorial/QuestSystem/UI/Wg_QuestNotification.Wg_QuestNotification_C" 0 _description))
    (UserInterface|Viewport|AddtoViewport _returnvalue 0)
    (bind _return (CallFunction|AreObjectivesComplete))
    (Variables|Default|SetIsCompleted _return)))

(fn AreObjectivesComplete
  (for _array_element (Utilities|Struct|BreakS_StageDetails (Variables|Default|GetCurrentStageDetails))
    (if (not (>= (.Value (Utilities|Map|Find (Variables|Default|GetCurrentObjectiveProgress) (Utilities|Struct|BreakS_ObjectiveDetails _array_element))) (.Quantiy (Utilities|Struct|BreakS_ObjectiveDetails (CallFunction|GetObjectiveDatabyID (Utilities|Struct|BreakS_ObjectiveDetails _array_element))))))
      (bind _output_get (LocalVariables|SetLocal_AllComplete false))
      (return _output_get)))
  (return (LocalVariables|GetLocal_AllComplete)))