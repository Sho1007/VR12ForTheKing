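; Quest log component that tracks active and completed quests by ID, with lookup for active status.
; Adding a quest records its ID and spawns a BP_QuestBase actor, stored for retrieval by ID.
; Turn-in only prints the current stage's XP reward, then completes the quest, moving its ID to completed and firing OnQuestCompleted.
; Completed quest actors stay in CurrentQuests, and TrackQuest is an empty stub.
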(event EventBeginPlay)

(event EventTick
  (params (DeltaSeconds :type Float%20%28single-precision%29)))

(fn AddNewQuest
  (params (QuestID :type Name))
  (Utilities|Array|AddUnique (Variables|Default|GetCurrentActiveQuests) QuestID)
  (bind _returnvalue (Game|SpawnActorfromClass "/Game/Develop/CH/QuestTutorial/Blueprints/BP_QuestBase.BP_QuestBase_C" (Math|Transform|MakeTransform "0, 0, 0" "0, 0, 0" "1.000000,1.000000,1.000000") "Undefined" 0 QuestID 0))
  (Utilities|Array|Add (Variables|Default|GetCurrentQuests) _returnvalue)
  (return _returnvalue))

(fn CompleteQuest
  (params (QuestID :type Name%20%28by%20ref%29))
  ;[1 1 1] 완료한 퀘스트에 대한 질문
  (Utilities|Array|AddUnique (Variables|Default|GetCompletedQuests) QuestID)
  (Utilities|Array|RemoveItem (Variables|Default|GetCurrentActiveQuests) QuestID)
  (bind _array_element (CallFunction|GetQuestActor QuestID))
  (Default|CallOnQuestCompleted _array_element))

(fn QueryActiveQuest
  (params (QuestID :type Name))
  (return (Utilities|Array|ContainsItem (Variables|Default|GetCurrentActiveQuests) QuestID)))

(fn TrackQuest)

(fn GetQuestActor
  (params (QuestID :type Name))
  ;[1 1 1] 퀘스트 엑터를 제대로 가져오는 것
  (for _array_element (Variables|Default|GetCurrentQuests)
    (if (== (Variables|/Game/Develop/CH/QuestTutorial/Blueprints/BP_QuestBase.BP_QuestBase_C|GetQuestID_Test _array_element) QuestID)
      (return _array_element))))

(fn TurninQuest
  (params (QuestID :type Name))
  (Utilities|FlowControl|Sequence
    (:then_0
      ;[1 1 1] 보상을 지급받는 방법
      (bind _array_element (CallFunction|GetQuestActor QuestID))
      (Development|PrintString (Utilities|String|ToString(Text) (Utilities|Text|FormatText "XP = {a}" (Utilities|Struct|BreakS_StageDetails (Variables|/Game/Develop/CH/QuestTutorial/Blueprints/BP_QuestBase.BP_QuestBase_C|GetCurrentStageDetails _array_element))))))
    (:then_1
      (CallFunction|CompleteQuest QuestID))))