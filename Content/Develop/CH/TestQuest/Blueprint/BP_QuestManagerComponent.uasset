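; Quest manager component that makes its owning actor an interaction point for a quest.
; InteractWith calls ActiveQuest on the game mode's QuestLogComponent with the first QuestArray entry, prints "Already on Quest" if true, and returns the owner's display name either way.
; Two functions marked as discarded read the current quest from QuestArray and reset the story index once it reaches the DT_QuestData story count.
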(fn DIscardDoNextQuest
  (bind _returnvalue (Utilities|GetDataTableRow "/Game/Develop/CH/Deta/DT_QuestData.DT_QuestData" (Utilities|Array|Get(acopy) (Variables|Default|GetQuestArray) (Variables|Default|GetCurrentQuestIndex)))
    (:then
      (if (== (Utilities|Array|Length (.storydataarray _returnvalue)) (Variables|Default|GetCurrentStoryIndex))
        (Variables|Default|SetCurrentStoryIndex 0)))))

(fn DIscardGetCurrentMainQuest
  (return (Utilities|Array|Get(acopy) (Variables|Default|GetQuestArray) (Variables|Default|GetCurrentQuestIndex))))

(fn Interactwith
  (bind _returnvalue (Components|GetOwner))
  (bind _returnvalue_2 (Utilities|GetDisplayName _returnvalue))
  (if (not (Default|ActiveQuest (Variables|/Game/Develop/CH/TestQuest/Blueprint/GM_TestQuest.GM_TestQuest_C|GetQuestLogComponent (CallFunction|GetMyGamemode)) (Utilities|Array|Get(acopy) (Variables|Default|GetQuestArray))))
    (return _returnvalue_2)
    (else
      (Development|PrintString "Already on Quest")
      (return _returnvalue_2))))