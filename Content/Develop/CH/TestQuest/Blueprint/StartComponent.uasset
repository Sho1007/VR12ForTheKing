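; StartComponent is a quest-giver component whose InteractWith checks the game mode's LogComponent for the configured quest and returns the owner's display name.
; If the quest is active it prints a notice; otherwise DisplayQuest runs.
; DisplayQuest feeds the quest's DataTable row into an NPC quest widget with UI-only input and a mouse cursor.
; It also creates event-info and on-screen widgets with hardcoded quest text, independent of that row.
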(event EventBeginPlay)

(event EventTick
  (params (DeltaSeconds :type Float%20%28single-precision%29)))

(fn DisplayQuest
  (bind _returnvalue (Game|GetPlayerController 0))
  (bind _dt_questdata (Variables|Default|GetDT_QuestData))
  (Utilities|FlowControl|Sequence
    (:then_0
      (bind _returnvalue_2 (Utilities|GetDataTableRow (.datatable _dt_questdata) (.rowname _dt_questdata))
        (:then
          (bind _returnvalue_3 (UserInterface|CreateWidget "/Game/Develop/CH/Widgets/Quest/WBP_NpcQuest.WBP_NpcQuest_C" 0 _returnvalue_2))
          (UserInterface|Viewport|AddtoViewport _returnvalue_3 0)
          (Utilities|IsValid _returnvalue
            (:Is%20Valid
              (Input|SetInputModeUIOnly _returnvalue _returnvalue_3 "DoNotLock" false)
              (Variables|/Script/Engine.PlayerController|SetbShowMouseCursor _returnvalue true))))))
    (:then_1
      (bind _returnvalue_4 (UserInterface|CreateWidget "/Game/Develop/CH/Widgets/Quest/WBP_QuestEventInfo.WBP_QuestEventInfo_C" 0 (Utilities|Struct|MakeS_QuestData "" "여기저기로 가세요")))
      (UserInterface|Viewport|AddtoViewport _returnvalue_4 0))
    (:then_2
      (bind _returnvalue_5 (UserInterface|CreateWidget "/Game/Develop/CH/Widgets/Quest/WBP_QuestOnScreen.WBP_QuestOnScreen_C" 0 (Utilities|Struct|MakeS_QuestData "" "여기저기로 가세요")))
      (UserInterface|Viewport|AddtoViewport _returnvalue_5 0))))

(fn Interactwith
  (bind _returnvalue (Components|GetOwner))
  (bind _returnvalue_2 (Utilities|GetDisplayName _returnvalue))
  (if (not (Default|ActiveQuest (Variables|/Game/Develop/CH/TestQuest/Blueprint/TestQuest_GM.TestQuest_GM_C|GetLogComponent (CallFunction|GetMyGamemode)) (.rowname (Variables|Default|GetDT_QuestData))))
    (CallFunction|DisplayQuest)
    (return _returnvalue_2)
    (else
      (Development|PrintString "Already on Quest")
      (return _returnvalue_2))))