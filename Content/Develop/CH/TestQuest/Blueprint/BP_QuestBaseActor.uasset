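; Quest base actor that loads a quest definition and holds the state for its first step.
; On BeginPlay it looks up its QuestID row in Discard_DT_QuestData and takes the first Purpose entry as the current quest data.
; It then resets CurrentStepProgress to a zero count per objective ObjectID.
; GetQuestDatabyID linearly searches those objectives for a matching ObjectID; nothing here advances progress.
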(event EventBeginPlay
  (CallFunction|GetQuestDetail))

(event Collision|EventActorBeginOverlap
  (params (OtherActor :type Actor%20Object%20Reference)))

(event EventTick
  (params (DeltaSeconds :type Float%20%28single-precision%29)))

(fn ConstructionScript)

(fn GetQuestDatabyID
  (params (QuestID :type String))
  (for _array_element (.Objective (Utilities|Struct|BreakDiscard_S_QuestData (Variables|Default|GetCurrentQuestData)))
    (if (Utilities|Enum|Equal(Enum) (Utilities|Struct|BreakDiscard_S_ObjectiveData _array_element) QuestID)
      (return _array_element))))

(fn GetQuestDetail
  (bind _returnvalue (Utilities|GetDataTableRow "/Game/Develop/CH/Deta/Discard_DT_QuestData.Discard_DT_QuestData" (Variables|Default|GetQuestID))
    (:then
      (bind _output_get (Variables|Default|SetQuestNPCData _returnvalue))
      (bind _output_get_2 (Variables|Default|SetCurrentQuestData (Utilities|Array|Get(acopy) (.Purpose (Utilities|Struct|BreakDiscard_S_QuestNPCData _output_get)))))
      (Utilities|Map|Clear (Variables|Default|GetCurrentStepProgress))
      (for _array_element (.Objective (Utilities|Struct|BreakDiscard_S_QuestData _output_get_2))
        (Utilities|Map|Add (Variables|Default|GetCurrentStepProgress) (.ObjectID (Utilities|Struct|BreakDiscard_S_ObjectiveData _array_element)) 0)))))