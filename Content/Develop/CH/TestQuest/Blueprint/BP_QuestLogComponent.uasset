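; BP_QuestLogComponent is a quest log component that starts, tracks and completes quests by QuestID.
; NewQuest records the ID in CurrentActiveQuest, spawns a BP_QuestBaseActor for it and stores that actor in CurrentQuest.
; GetQuestActor searches those actors by ID, and ActiveQuest checks whether an ID is active.
; Complete fires the quest actor's OnQuestComplete, but adds the ID to CurrentActiveQuest and removes it from CompleteQuest, apparently reversed.
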(event EventBeginPlay)

(event EventTick
  (params (DeltaSeconds :type Float%20%28single-precision%29)))

(fn NewQuest
  (params (QuestID :type Name%20%28by%20ref%29))
  (Utilities|Array|AddUnique (Variables|Default|GetCurrentActiveQuest) QuestID)
  (bind _returnvalue (Game|SpawnActorfromClass "/Game/Develop/CH/TestQuest/Blueprint/BP_QuestBaseActor.BP_QuestBaseActor_C" (Math|Transform|MakeTransform "0, 0, 0" "0, 0, 0" "1.000000,1.000000,1.000000") "Undefined" 0 QuestID 0))
  (Utilities|Array|Add (Variables|Default|GetCurrentQuest) _returnvalue)
  (return _returnvalue))

(fn GetQuestActor
  (params (QuestID :type Name))
  (for _array_element (Variables|Default|GetCurrentQuest)
    (if (== (Variables|/Game/Develop/CH/TestQuest/Blueprint/BP_QuestBaseActor.BP_QuestBaseActor_C|GetQuestID _array_element) QuestID)
      (return _array_element))))

(fn Complete
  (params (QuestID :type Name%20%28by%20ref%29))
  ;[1 1 1] 완료 되었는가
  (Utilities|Array|AddUnique (Variables|Default|GetCurrentActiveQuest) QuestID)
  (Utilities|Array|RemoveItem (Variables|Default|GetCompleteQuest) QuestID)
  (bind _array_element (CallFunction|GetQuestActor QuestID))
  (Default|CallOnQuestComplete _array_element))

(fn ActiveQuest
  (params (QuestID :type Name))
  ;[1 1 1] 활성화된 퀘스트가 있는지 확인
  (return (Utilities|Array|ContainsItem (Variables|Default|GetCurrentActiveQuest) QuestID)))