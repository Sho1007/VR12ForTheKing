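; BP_DynamicCamera is a spring-arm camera actor that can orbit and either follow an actor or move to a location.
; SetOrbit toggles RotatingMovement and spring-arm yaw inheritance, resetting actor rotation when off.
; SetDynamicLocation attaches to a valid actor, otherwise stores a target vector without detaching.
; While unattached, Tick sets location through VInterpTo with Current and Target reversed, landing near the target instead of easing toward it.
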(event EventSetDynamicLocation
  (params (Actor :type Actor%20Object%20Reference) (Vector :type Vector :default "0, 0, 0"))
  (Utilities|IsValid Actor
    (:Is%20Valid
      (Transformation|AttachActorToActor Actor "None" "SnapToTarget" "KeepWorld" "KeepWorld" true)
      (Transformation|SetRelativeRotation (Variables|Default|GetCamera) "0, 0, 0" false false))
    (:Is%20Not%20Valid
      (Variables|Default|SetTargetLoaction Vector))))

(event EventSetOrbit
  (params (Orbiting :type Boolean))
  (Variables|/Script/Engine.RotatingMovementComponent|SetRotationRate (Variables|Default|GetRotatingMovement) (Math|Rotator|SelectRotator "0.000000,10.000000,0.000000" "0, 0, 0" Orbiting))
  (bind _output_get (Variables|/Script/Engine.SpringArmComponent|SetbInheritYaw (Variables|Default|GetSpringArm) Orbiting))
  (if (not _output_get)
    (Transformation|SetActorRotation "0, 0, 0")))

(event EventTick
  (params (DeltaSeconds :type Float%20%28single-precision%29))
  (Utilities|IsValid (Actor|GetAttachParentActor)
    (:Is%20Not%20Valid
      (Transformation|SetActorLocation (Math|Interpolation|VInterpTo (Variables|Default|GetTargetLoaction) (Transformation|GetActorLocation) (Utilities|Time|GetWorldDeltaSeconds) 5.0) false false))))

(fn ConstructionScript)