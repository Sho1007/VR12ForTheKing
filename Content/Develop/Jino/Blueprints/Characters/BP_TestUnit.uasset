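; BP_TestUnit is a test unit Blueprint that exercises the top info HUD and its move-turn widgets.
; On BeginPlay it creates WBP_TopInfoWidget, adds it to the viewport and initializes the move-turn and nested character turn widgets.
; Debug key G calls Test, which updates the character turn widget, passes the result to MoveToNextDay, then calls ChaosCount and GetDayText.
; Battle turn widget initialization is left unconnected.
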(event EventBeginPlay
  (|CallParentFunction)
  (bind _returnvalue (UserInterface|CreateWidget "/Game/Develop/Jino/Blueprints/Widgets/ActionWidget/TopInfoWidget/WBP_TopInfoWidget.WBP_TopInfoWidget_C"))
  (bind _output_get (Variables|Default|SetNewVar _returnvalue))
  (UserInterface|Viewport|AddtoViewport _output_get 0)
  (Class|MoveTurnWidget|InitTurnWidget (Variables|/Game/Develop/Jino/Blueprints/Widgets/ActionWidget/TopInfoWidget/WBP_TopInfoWidget.WBP_TopInfoWidget_C|GetWBP_MoveTurnWidget _returnvalue) 1)
  (Class|CharacterTurnWidget|InitWidget (Variables|/Game/Develop/Jino/Blueprints/Widgets/ActionWidget/TopInfoWidget/MoveTurnWidget/WBP_MoveTurnWidget.WBP_MoveTurnWidget_C|GetWBP_CharacterTurnWidget (Variables|/Game/Develop/Jino/Blueprints/Widgets/ActionWidget/TopInfoWidget/WBP_TopInfoWidget.WBP_TopInfoWidget_C|GetWBP_MoveTurnWidget _returnvalue))))

(event Input|KeyboardEvents|DebugKeyG
  (params (Key :type Key%20Structure :default "None") (ActionValue :type Input%20Action%20Value%20Structure))
  (:Pressed
    (CallFunction|Test)))

(fn ConstructionScript
  (|CallParentFunction))

(fn Test
  (bind _newvar (Variables|Default|GetNewVar))
  (bind _wbp_moveturnwidget (Variables|/Game/Develop/Jino/Blueprints/Widgets/ActionWidget/TopInfoWidget/WBP_TopInfoWidget.WBP_TopInfoWidget_C|GetWBP_MoveTurnWidget _newvar))
  (bind _returnvalue (Class|CharacterTurnWidget|UpdateWidget (Variables|/Script/VR12ForTheKing.MoveTurnWidget|GetWBP_CharacterTurnWidget _wbp_moveturnwidget)))
  (Class|MoveTurnWidget|MovetoNextDay _wbp_moveturnwidget _returnvalue)
  (Class|TurnWidget|ChaosCount _newvar)
  (Class|TurnWidget|GetDayText _newvar))