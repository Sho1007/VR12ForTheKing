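; BP_Projectile is a projectile that damages a designated AttackTarget once it gets close enough.
; On BeginPlay its Sphere ignores the instigator while moving.
; Each Tick it measures distance to the target instead of using overlap events, and within HitRange applies Damage with DamageTypeClass, prints debug text and destroys itself.
; The ImpactEffect emitter spawn is unconnected, so no impact effect plays from this graph.
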(event EventBeginPlay
  (Collision|IgnoreActorwhenMoving (Variables|Default|GetSphere) (Game|GetInstigator) true))

(event Collision|EventActorBeginOverlap
  (params (OtherActor :type Actor%20Object%20Reference)))

(event EventTick
  (params (DeltaSeconds :type Float%20%28single-precision%29))
  (if (<= (Math|Vector|Distance(Vector) (Transformation|GetActorLocation (Variables|Default|GetAttackTarget)) (Transformation|GetActorLocation)) (Variables|Default|GetHitRange))
    (Development|PrintString (Utilities|String|Append "damage:" (Utilities|String|ToString(Float) (Variables|Default|GetDamage))))
    (Game|Damage|ApplyDamage (Variables|Default|GetAttackTarget) (Variables|Default|GetDamage) 0 0 (Variables|Default|GetDamage%20Type%20Class))
    (Development|PrintString "applied damage")
    (Actor|DestroyActor)))

(fn ConstructionScript)