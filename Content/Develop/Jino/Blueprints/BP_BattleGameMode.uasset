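; BP_BattleGameMode runs a turn-based battle, setting up the camera, unit lists and HUD, and sequencing unit turns.
; BeginPlay switches to the top-down camera, gathers party and enemy units, then after a short delay adds party units to the BattlePC's HUD.
; TurnRequest queues units uniquely, and a DoOnce gate in StartTurn starts the first unit's turn through its BattleComponent.
; It binds to TurnEnded, and ReadyNextTurn reopens the gate for the next queued unit.
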(event Custom|TurnRequest
  (params (Unit :type BP%20Unit%20Base%20Object%20Reference))
  ;[1 1 1] TurnRequest가 호출되면 TurnOrder배열에 unitbase타입의 액터를 중복되지 않게 추가 그리고 StartTurn을 호출한다.
  (Utilities|Array|AddUnique (Variables|Default|GetTurnOrder) Unit)
  (CallFunction|StartTurn))

(event Custom|StartTurn
  (Development|PrintString "StartTurn")
  (Utilities|FlowControl|DoOnce false
    (:Completed
      (if (Utilities|Array|IsValidIndex (Variables|Default|GetTurnOrder))
        ;[1 1 1] TurnOrder배열의 0번째 요소를 가지고 combatcomponent에 있는 StartUnit을 호출한다.
        (bind _asbp_battle_component (Utilities|Casting|CastToBP_BattleComponent (Variables|/Script/VR12ForTheKing.MyCharacter|GetBattleComponent (Utilities|Array|Get(acopy) (Variables|Default|GetTurnOrder)))))
        (Default|StartUnitTurn _asbp_battle_component)
        ;[1 1 1] turn order배열에서 0번째 요소 제거 디스패처를 통해 ReadyNextTurn이벤트 호출?
        (EventDispatchers|BindEventtoTurnEnded _asbp_battle_component (EventDispatchers|CreateEvent :!event Custom|ReadyNextTurn))
        (Utilities|Array|RemoveIndex (Variables|Default|GetTurnOrder))
        (else
          ;[1 1 1] 지금 턴을 진행중인 유닛의 턴이 끝나기 전까지 다음유닛의 턴이 오지않게 대기시키는 코드
          (CallFunction|ReadyNextTurn))))))

(event Custom|ReadyNextTurn
  ;[1 1 1] 지금 턴을 진행중인 유닛의 턴이 끝나기 전까지 다음유닛의 턴이 오지않게 대기시키는 코드
  (Utilities|FlowControl|Sequence
    (:then_0
      (Utilities|FlowControl|DoOnce false) ; enters at Reset
    )
    (:then_1
      (if (Utilities|Array|IsValidIndex (Variables|Default|GetTurnOrder))
        (CallFunction|StartTurn)))))

(event EventBeginPlay
  ;[1 1 1] 게임이 시작되면 Camera_TopDown클래스의 MainBattleCamera시점으로 PlayerController의 시점이 이동한다
  (bind _returnvalue (Actor|GetActorOfClass "/Game/Develop/Jino/Blueprints/Cameras/Camera_TopDown.Camera_TopDown_C"))
  (bind _output_get (Variables|Default|SetMain%20Battle%20Camera _returnvalue))
  (Game|Player|SetViewTargetwithBlend (Game|GetPlayerController 0) _output_get 0.0 "VTBlend_Linear" 0.0 false)
  ;[1 1 1] PartyUnitBase클래스타입의 액터들을 모두 PartyUnits배열에 넣는다
  (bind _outactors (Actor|GetAllActorsOfClass "/Game/Develop/Jino/Blueprints/BP_PartyUnitBase.BP_PartyUnitBase_C"))
  (Variables|Default|SetParty%20Units _outactors)
  ;[1 1 1] EnemyUnitBase타입의 액터들을 전부 Enemy Units클래스에 넣는다
  (bind _outactors_2 (Actor|GetAllActorsOfClass "/Game/Develop/Jino/Blueprints/BP_EnemyUnitBase.BP_EnemyUnitBase_C"))
  (Variables|Default|SetEnemy%20Units _outactors_2)
  (Utilities|FlowControl|Delay 0.2)
  ;[1 1 1] BattlePC에서 BattleHud를 받아와서 PartyUnit을 input으로 받는  BattleHud의 AddPartyUnit to Hud 함수를 호출
  (bind _asbp_battle_pc (Utilities|Casting|CastToBP_BattlePC (Game|GetPlayerController 0)))
  (Variables|Default|SetBattle%20Hud (Variables|/Game/Develop/Jino/Blueprints/BP_BattlePC.BP_BattlePC_C|GetBattleHud _asbp_battle_pc))
  (for _array_element (Variables|Default|GetParty%20Units)
    (Default|AddPartyUnittoHUD (Variables|Default|GetBattle%20Hud) _array_element)))

(fn ConstructionScript)