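; Battle component for a unit in a timer-driven turn-based battle, handling turn timing, actions and damage or healing math.
; A Speed-scaled timer requests a turn from BP_BattleGameMode, then party units get a command HUD while others pick a random action, with an orbit camera on the active unit.
; Melee approaches the target, ranged and spells spawn actors, and returning to the battle position ends the turn and restarts the timer.
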(event Custom|AttackCommand
  ;[1 1 1] 카메라가 유닛을따라다니도록
  ;;[1 0 0.04958] Turn이 넘어가면 카메라도 Orbit을 실행해야하는데 한번씩 멈춤
  (Class|BPDynamicCameraIT|SetOrbit(Message) (Pawn|GetViewTarget (Game|GetPlayerController 0)) false)
  ;[1 1 1] 근거리 원거리 유닛타입에 따라 공격방식이 다름
  (CallFunction|DiscardMeleeAttack))

(event Custom|ReachToDesination
  ;[1 1 1] 유닛이 목표에 접근했다가 다시 원래 위치로 돌아오는 로직
  (Actor|Tick|SetActorTickEnabled (Components|GetOwner))
  (if (not (Variables|Default|GetDiscard_Turn%20end))
    (if (Variables|Default|GetDiscard_GoBack)
      ;;[1 0 0.07212] 가끔씩 턴이 넘어가지않고 유닛이 떨리는 현상이 발생함
      (CallFunction|DiscardBacktoBattlePos)
      (else
        (CallFunction|Reached)))))

(event Custom|Discard_RangeAttack
  (bind _unitcharacter (Variables|Default|GetUnitCharacter))
  (bind _unitcharacter_2 (Variables|Default|GetUnitCharacter))
  ;[1 1 1] 원거리 공격 - 정해진 위치로 이동후 공격해니메이션 실행하고 원래자리에 돌아온다. 공격이 끝나면 유닛의 턴이 끝나고 다음턴으로 이어짐
  (Variables|Default|SetDiscard_Turn%20end false)
  (Transformation|SetActorRotation _unitcharacter_2 (Math|Rotator|FindLookatRotation (Transformation|GetActorLocation _unitcharacter_2) (Transformation|GetActorLocation (Variables|Default|GetUnitTarget))))
  (bind _basedamage (CallFunction|DiscardCalculateDamage))
  (Game|SpawnActorfromClass (Variables|Default|GetProjectileClass) (Transformation|GetActorTransform _unitcharacter) "AdjustIfPossibleButAlwaysSpawn" 0 (Variables|Default|GetUnitTarget) _basedamage _unitcharacter)
  (Utilities|Time|SetTimerbyFunctionName 0 "BacktoBattlePos" 2.0)
  (Variables|Default|SetIsRangeAttack false)
  (bind _actioncommandwindow (Variables|Default|GetActionCommandWindow)
    (:then
      (Widget|RemovefromParent _actioncommandwindow))
    (:else)))

(event Custom|Discard_MeleeAttack
  ;[1 1 1] 근접공격 - 적에게 접근해서 공격해니메이션 실행하고 원래자리에 돌아온다. 공격이 끝나면 유닛의 턴이 끝나고 다음턴으로 이어짐
  (Variables|Default|SetDiscard_Turn%20end false)
  (bind _asbp_unit_base (Utilities|Casting|CastToBP_UnitBase (Components|GetOwner)))
  (Transformation|SetActorRotation _asbp_unit_base (Math|Rotator|FindLookatRotation (Transformation|GetActorLocation _asbp_unit_base) (Transformation|GetActorLocation (Variables|Default|GetUnitTarget))))
  (Class|MyCharacter|SetDestination _asbp_unit_base (Transformation|GetActorLocation (Variables|Default|GetUnitTarget)) 0.0 5.0)
  (bind _actioncommandwindow (Variables|Default|GetActionCommandWindow)
    (:then
      (Widget|RemovefromParent _actioncommandwindow))
    (:else)))

(event Custom|MagicCommand
  (params (SpellType :type BP%20Magic%20Base%20Class%20Reference))
  ;[1 1 1] 마법사용
  (Class|BPDynamicCameraIT|SetOrbit(Message) (Pawn|GetViewTarget (Game|GetPlayerController 0)) false)
  (if (Utilities|ClassIsChildOf SpellType "/Game/Develop/Jino/Blueprints/Abilities/BlackMagic/BP_BlackMagicBase.BP_BlackMagicBase_C")
    (CallFunction|CastBlackMagic SpellType)))

(event Custom|CastBlackMagic
  (params (BlackMagicSpell :type BP%20Magic%20Base%20Class%20Reference))
  (bind _unitcharacter (Variables|Default|GetUnitCharacter))
  (bind _unittarget (Variables|Default|GetUnitTarget))
  ;[1 1 1] 적방향으로 쳐다보게
  (Development|PrintString "Use BlackMagic" true true "(R=0.000000,G=0.660000,B=1.000000,A=1.000000)" 6e+01)
  (Variables|Default|SetBlack%20Magic%20Spell BlackMagicSpell)
  (Transformation|SetActorRotation _unitcharacter (Math|Rotator|FindLookatRotation (Transformation|GetActorLocation _unitcharacter) (Transformation|GetActorLocation (Variables|Default|GetUnitTarget))))
  ;[1 1 1] Comment
  (bind _returnvalue (CallFunction|CalculateMagicBaseDamage (Variables|Default|GetBlack%20Magic%20Spell)))
  ;[1 1 1] BlackMagicSpell클래스 액터의 스폰위치는 TargetUnit의 위치
  (Game|SpawnActorfromClass (Variables|Default|GetBlack%20Magic%20Spell) (Transformation|GetActorTransform _unittarget) "AdjustIfPossibleButAlwaysSpawn" 0 _unittarget _returnvalue (Variables|Default|GetUnitCharacter))
  (Utilities|Time|SetTimerbyFunctionName 0 "SetDestinationToBattlePos" 2.0)
  (bind _actioncommandwindow (Variables|Default|GetActionCommandWindow)
    (:then
      (Widget|RemovefromParent _actioncommandwindow))
    (:else)))

(event Custom|EndBlackMagic
  (params (NewParam :type Actor%20Object%20Reference) (NewParam2 :type EEndPlayReason%20Enum :default "Destroyed"))
  ;[1 1 1] 공격마법
)

(event Custom|RangeAttackCommand
  (Variables|Default|SetIsRangeAttack true)
  (Class|BPDynamicCameraIT|SetOrbit(Message) (Pawn|GetViewTarget (Game|GetPlayerController 0)) false)
  (CallFunction|DiscardRangeAttack))

(event EventBeginPlay
  ;[1 1 1] 게임이 시작됐을 때 유닛들을 해당 유닛스폰위치에 스폰
  (bind _asbp_unit_base (Utilities|Casting|CastToBP_UnitBase (Components|GetOwner)))
  (bind _output_get (Variables|Default|SetUnitCharacter _asbp_unit_base))
  (Variables|Default|SetDiscard_BattlePostion (Transformation|GetActorTransform _output_get))
  (CallFunction|BegineBattle)
  ;[1 1 1] 레벨에 따른 유닛들의 스텟설정 이단계에서는 아직 레벨이 같다면 모든 유닛의 스텟이 똑같다
  (bind _returnvalue (Utilities|GetDataTableRow "/Game/Develop/Jino/Blueprints/Data/BaseStatTable.BaseStatTable" (Utilities|String|StringToName (Utilities|String|ToString(Integer) (Variables|UnitStats|GetUnitLevel))))
    (:then
      (Variables|UnitStats|SetBaseUnitStat _returnvalue))))

(fn StartUnitTurn
  ;[1 1 1] StartUnitTurn함수가 호출되면 UnitCharacter가 PartyUnitBase클래스의 자식클래스인지를 확인해라
  (if (Utilities|ClassIsChildOf (Utilities|GetClass (Variables|Default|GetUnitCharacter)) "/Game/Develop/Jino/Blueprints/BP_PartyUnitBase.BP_PartyUnitBase_C")
    ;[1 1 1] PartyUnit의 자식클래스 가 맞다면 unit character의 actioncommand widget을 화면에 추가하고 set camera함수 호출
    (bind _returnvalue (UserInterface|CreateWidget "/Game/Develop/Jino/Blueprints/Widgets/BP_UnitBattleHud.BP_UnitBattleHud_C" 0 (Variables|Default|GetUnitCharacter)))
    (bind _output_get (Variables|Default|SetActionCommandWindow _returnvalue))
    (UserInterface|Viewport|AddtoViewport _output_get 0)
    (CallFunction|SetCamera)
    (else
      (bind _outactors (Actor|GetAllActorsOfClass "/Game/Develop/Jino/Blueprints/BP_PartyUnitBase.BP_PartyUnitBase_C"))
      (Variables|Default|SetUnitTarget (.OutItem (Utilities|Array|Random _outactors)))
      (switch int 0
        (:0
          (CallFunction|RandomBattleAction)
          (CallFunction|SetCamera))))))

(fn BegineBattle
  (bind _unitcharacter (Variables|Default|GetUnitCharacter))
  (bind _maxactiontime (Variables|UnitStats|GetMaxActionTime))
  (bind _minactiontime (Variables|UnitStats|GetMinActionTime))
  (bind _minactiontime_2 (Variables|UnitStats|GetMinActionTime))
  (bind _returnvalue (Actor|GetComponentbyClass _unitcharacter "/Script/VR12ForTheKing.StatusComponent"))
  (bind _returnvalue_2 (- _maxactiontime _minactiontime))
  (bind _characterstatus (Variables|/Script/VR12ForTheKing.StatusComponent|GetCharacterStatus _returnvalue))
  (bind _returnvalue_3 (Math|Conversions|ToFloat(Integer) (.speed _characterstatus)))
  (bind _returnvalue_4 (Math|Float|NormalizetoRange _returnvalue_3 0.0 255.0))
  (bind _returnvalue_5 (- 1.0 _returnvalue_4))
  (bind _returnvalue_6 (* _returnvalue_5 _returnvalue_2))
  (bind _returnvalue_7 (+ _returnvalue_6 _minactiontime_2))
  (Utilities|IsValid _returnvalue
    (:Is%20Valid
      ;[1 1 1] 턴을 분배하는 공식 속도가 빠를수록 먼저 턴이 돌아온다.
      (Development|PrintString (Utilities|String|ToString(Float) _returnvalue_7))
      (bind _returnvalue_8 (Utilities|Time|SetTimerbyFunctionName self "RequestTurn" _returnvalue_7))
      (Variables|Default|SetActionTimer _returnvalue_8))))

(fn EndUnitTurn
  ;[1 1 1] 턴이 끝나으면 BegineBattle을 호출해서 다음유닛의 턴이 오게함
  (Default|CallTurnEnded)
  (CallFunction|BegineBattle))

(fn RequestTurn
  (bind _unitcharacter (Variables|Default|GetUnitCharacter))
  (bind _asbp_battle_game_mode (Utilities|Casting|CastToBP_BattleGameMode (Game|GetGameMode)))
  (Development|PrintString (Utilities|String|Append (Utilities|GetDisplayName _unitcharacter) "Turn") true true "(R=0.000000,G=0.660000,B=1.000000,A=1.000000)" 6e+01)
  (Default|TurnRequest _asbp_battle_game_mode _unitcharacter))

(fn SetCamera
  (bind _returnvalue (Actor|GetActorOfClass "/Game/Develop/Jino/Blueprints/Cameras/BP_DynamicCamera.BP_DynamicCamera_C"))
  (Game|Player|SetViewTargetwithBlend (Game|GetPlayerController 0) _returnvalue 0.0 "VTBlend_Linear" 0.0 false)
  (Class|BPDynamicCameraIT|SetDynamicLocation(Message) _returnvalue (Variables|Default|GetUnitCharacter) "0, 0, 0")
  (Development|PrintString "Hello")
  (Class|BPDynamicCameraIT|SetOrbit(Message) (Pawn|GetViewTarget (Game|GetPlayerController 0)) true))

(fn DiscardCalculateDamage
  (bind _calculateddamage (CallFunction|CalculateBaseDamage))
  (return _calculateddamage))

(fn GetRangePosition
  (bind _unitcharacter (Variables|Default|GetUnitCharacter))
  (bind _returnvalue (Transformation|GetActorLocation _unitcharacter))
  (return (+ _returnvalue (* (Math|Vector|GetUnitDirection(Vector) _returnvalue (Transformation|GetActorLocation (Variables|Default|GetUnitTarget))) 5e+02))))

(fn CalculateBaseDamage
  (params (NewParam :type Integer))
  ;[1 1 1] Unit의 Strength계수에 기본스텟을 곲하고 거기에 기본데미지값(5)에 데미지가 항상같게 나오지않게 랜덤값을 곱해서 반환
  (return (Math|Random|RandomFloatinRange 0.9 1.1)))

(fn CalculateDamageResistance
  (params (BaseDamage :type Float%20%28double-precision%29))
  ;[1 1 1] 들어온데미지를 제곱한것에 저항값으로 나눠서 캐릭터마다 다른 데미지가 들어오게
  (return (/ (Math|Float|Power BaseDamage 2.0) (+ BaseDamage (.armor (Variables|/Script/VR12ForTheKing.StatusComponent|GetCharacterStatus (Actor|GetComponentbyClass (Variables|Default|GetUnitCharacter) "/Script/VR12ForTheKing.StatusComponent")))))))

(fn Reached
  (Development|PrintString "reached success" true true "(R=0.000000,G=0.660000,B=1.000000,A=1.000000)" 6e+01)
  (Variables|Default|SetAttackDamageOnce true)
  (if (Variables|Default|GetAttackDamageOnce)
    (CallFunction|DoMeleeAttack)
    (Variables|Default|SetDiscard_GoBack true)
    (CallFunction|SetDestinationtoBattlePos)))

(fn DiscardBacktoBattlePos
  ;[1 1 1] 원래 위치로 돌아올때 유닛의 보는 방향도 처음과 같게 하기, 돌아온다음에는 턴 끝내기
  (Development|PrintString "turnend")
  (Transformation|SetActorRotation (Variables|Default|GetUnitCharacter) (.Rotation (Math|Transform|BreakTransform (Variables|Default|GetDiscard_BattlePostion))))
  (Variables|Default|SetDiscard_GoBack false)
  (Variables|Default|SetDiscard_Turn%20end true)
  (Utilities|Time|SetTimerbyFunctionName 0 "EndUnitTurn" 2.0))

(fn SetDestinationtoBattlePos
  (bind _asbp_unit_base (Utilities|Casting|CastToBP_UnitBase (Components|GetOwner)))
  (Class|MyCharacter|SetDestination _asbp_unit_base (.Location (Math|Transform|BreakTransform (Variables|Default|GetDiscard_BattlePostion))) 0.0 1.0))

(fn DoMeleeAttack
  (bind _asbp_unit_base (Utilities|Casting|CastToBP_UnitBase (Components|GetOwner)))
  (bind _basedamage (CallFunction|DiscardCalculateDamage))
  (bind _asbp_battle_component (Utilities|Casting|CastToBP_BattleComponent (Variables|/Script/VR12ForTheKing.MyCharacter|GetBattleComponent _asbp_unit_base)))
  (Development|PrintString (Utilities|String|Append "damage:" (Utilities|String|ToString(Float) _basedamage)))
  (Game|Damage|ApplyDamage (Variables|BP_BattleComponent_C|GetUnitTarget _asbp_battle_component) _basedamage 0 _asbp_unit_base (Variables|Default|GetDamage%20Type%20Class))
  (Variables|Default|SetAttackDamageOnce false))

(fn CalculateMagicBaseDamage
  (params (SpellRank :type BP%20Magic%20Base%20Class%20Reference))
  (bind _returnvalue (Math|Random|RandomFloatinRange 0.9 1.1))
  (bind (_abilityname _rank _spelltarget _spellpowertable) (Utilities|GetClassDefaults SpellRank))
  (bind _unitcharacter (Variables|Default|GetUnitCharacter))
  (bind _value (Utilities|Map|Find _spellpowertable _rank))
  (bind _returnvalue_2 (Actor|GetComponentbyClass _unitcharacter "/Script/VR12ForTheKing.StatusComponent"))
  (bind _returnvalue_3 (Math|Float|Sqrt _value))
  (bind _characterstatus (Variables|/Script/VR12ForTheKing.StatusComponent|GetCharacterStatus _returnvalue_2))
  (bind _returnvalue_4 (* _returnvalue_3 2.0))
  (bind _returnvalue_5 (* (.intelligence _characterstatus) _returnvalue_4))
  (bind _returnvalue_6 (* _returnvalue_5 _returnvalue))
  (Development|PrintString "calculate Damage" true true "(R=0.000000,G=0.660000,B=1.000000,A=1.000000)" 6e+01)
  (Development|PrintString (Utilities|String|Append "Magic Rank: " (Utilities|GetClassDisplayName SpellRank)) true true "(R=0.000000,G=0.660000,B=1.000000,A=1.000000)" 6e+01)
  (Development|PrintString (Utilities|String|Append "MagicDamage:" (Utilities|String|ToString(Float) _returnvalue_6)) true true "(R=0.000000,G=0.660000,B=1.000000,A=1.000000)" 6e+01)
  (return _returnvalue_6))

(fn GetTurnSpeed
  (params (CurrentRoundCount :type Integer) (Speed :type Integer))
  (return (Math|Float|Truncate (* (/ CurrentRoundCount Speed) 1e+02))))

(fn ActionArrayMeleeAttack
  (|CallParentFunction)
  (Development|PrintString "MeleeAttack" true true "(R=0.000000,G=0.660000,B=1.000000,A=1.000000)" 6e+01)
  (bind _asmy_game_mode_base (Utilities|Casting|CastToMyGameModeBase (Game|GetGameMode)))
  (switch Utilities|FlowControl|Switch|SwitchonEFactionType (Variables|Default|GetFactionType)
    (:Player
      (bind _actiontarget (Variables|Default|GetActionTarget)
        (:then
          _)
        (:else)))
    (:Enemy
      (Variables|Default|SetActionTarget (.OutItem (Utilities|Array|Random (Variables|/Script/VR12ForTheKing.MyGameModeBase|GetCharacterArray _asmy_game_mode_base))))))
  (if (Utilities|Enum|NotEqual(Enum) (Variables|/Script/VR12ForTheKing.BattleComponent|GetFactionType (Variables|/Script/VR12ForTheKing.MyCharacter|GetBattleComponent _actiontarget)) (Variables|Default|GetFactionType))
    (Development|PrintString "DoMeleeAttack")
    (CallFunction|DiscardMeleeAttack)
    (return)
    (else
      (Development|PrintString "Can not Attack Your Faction")
      (return))))

(fn RandomBattleAction
  (bind _actionarray (Variables|Default|GetActionArray))
  (|CallParentFunction)
  (Development|PrintString "Called Battle Action")
  (Development|PrintString (Utilities|String|ToString(Integer) (Utilities|Array|Length _actionarray)))
  (bind _output_get (LocalVariables|SetNewAction (.OutItem (Utilities|Array|Random _actionarray))))
  (if (== _output_get "NormalAttack")
    (Development|PrintString "DoActionArrayAttack" true true "(R=0.000000,G=0.660000,B=1.000000,A=1.000000)" 6e+01)
    (CallFunction|ActionArrayMeleeAttack)
    (elif (== _output_get "WeakHeal")
      (Development|PrintString "DoWeakHeal" true true "(R=0.000000,G=0.660000,B=1.000000,A=1.000000)" 6e+01)
      (CallFunction|ActionArrayWeakHeal)
      (elif (== _output_get "RangeAttack")
        (Development|PrintString "DoActionArrayRangeAttack" true true "(R=0.000000,G=0.660000,B=1.000000,A=1.000000)" 6e+01)
        (CallFunction|ActionArrayRangeAttack)
        (elif (== _output_get "RandomMagic")
          (Development|PrintString "UseRandomMagic" true true "(R=0.000000,G=0.660000,B=1.000000,A=1.000000)" 6e+01)
          (CallFunction|ActionArrayRandomMagic)
          (else
            (Development|PrintString "error" true true "(R=0.000000,G=0.660000,B=1.000000,A=1.000000)" 6e+01)))))))

(fn ActionArrayRangeAttack
  (|CallParentFunction)
  (Development|PrintString "Doing rangedattack" true true "(R=0.000000,G=0.660000,B=1.000000,A=1.000000)" 6e+01)
  (bind _asmy_game_mode_base (Utilities|Casting|CastToMyGameModeBase (Game|GetGameMode)))
  (switch Utilities|FlowControl|Switch|SwitchonEFactionType (Variables|Default|GetFactionType)
    (:Player
      (bind _actiontarget (Variables|Default|GetActionTarget)
        (:then
          _)
        (:else)))
    (:Enemy
      (Variables|Default|SetActionTarget (.OutItem (Utilities|Array|Random (Variables|/Script/VR12ForTheKing.MyGameModeBase|GetCharacterArray _asmy_game_mode_base))))))
  (if (Utilities|Enum|NotEqual(Enum) (Variables|/Script/VR12ForTheKing.BattleComponent|GetFactionType (Variables|/Script/VR12ForTheKing.MyCharacter|GetBattleComponent _actiontarget)) (Variables|Default|GetFactionType))
    (CallFunction|DiscardRangeAttack)
    (return)
    (else
      (Development|PrintString "Can not Attack Your Faction")
      (return))))

(fn Heal
  (params (HealTarget :type BP%20Unit%20Base%20Object%20Reference))
  (bind _unitcharacter (Variables|Default|GetUnitCharacter))
  (Utilities|IsValid (Actor|GetComponentbyClass HealTarget "/Script/VR12ForTheKing.StatusComponent")
    (:Is%20Valid
      (Development|PrintString "Use WeakHeal" true true "(R=0.000000,G=0.660000,B=1.000000,A=1.000000)" 6e+01)
      (Transformation|SetActorRotation _unitcharacter (Math|Rotator|FindLookatRotation (Transformation|GetActorLocation _unitcharacter) (Transformation|GetActorLocation HealTarget)))
      ;[1 1 1] Comment
      (bind _healamount (CallFunction|CalculateBaseHeal))
      (Game|SpawnActorfromClass "/Game/Develop/Jino/Blueprints/Abilities/WhiteMagic/BP_WeakHeal.BP_WeakHeal_C" (Transformation|GetActorTransform HealTarget) "AdjustIfPossibleButAlwaysSpawn" 0 _healamount (Variables|Default|GetUnitCharacter))
      (Utilities|Time|SetTimerbyFunctionName 0 "SetDestinationToBattlePos" 2.0))))

(fn ActionArrayWeakHeal
  (Development|PrintString "Doing weakHeal" true true "(R=0.000000,G=0.660000,B=1.000000,A=1.000000)" 6e+01)
  (bind _asmy_game_mode_base (Utilities|Casting|CastToMyGameModeBase (Game|GetGameMode)))
  (switch Utilities|FlowControl|Switch|SwitchonEFactionType (Variables|Default|GetFactionType)
    (:Player
      (bind _actiontarget (Variables|Default|GetActionTarget)
        (:then
          (if (Utilities|Enum|NotEqual(Enum) (Variables|/Script/VR12ForTheKing.BattleComponent|GetFactionType (Variables|/Script/VR12ForTheKing.MyCharacter|GetBattleComponent _actiontarget)) (Variables|Default|GetFactionType))
            (Development|PrintString "Can not Heal Apponent Faction" true true "(R=0.000000,G=0.660000,B=1.000000,A=1.000000)" 6e+01)
            (return)
            (else
              _)))
        (:else)))
    (:Enemy
      ;[1 1 1] TempTarget
      (bind _asbp_battle_game_mode (Utilities|Casting|CastToBP_BattleGameMode (Game|GetGameMode)))))
  (CallFunction|Heal (.OutItem (Utilities|Array|Random (Variables|/Game/Develop/Jino/Blueprints/BP_BattleGameMode.BP_BattleGameMode_C|GetEnemy%20Units _asbp_battle_game_mode))))
  (return))

(fn CalculateBaseHeal
  (params (NewParam :type Integer))
  (bind _returnvalue (Math|Random|RandomFloatinRange 0.9 1.1))
  (bind _unitcharacter (Variables|Default|GetUnitCharacter))
  (bind _returnvalue_2 (Actor|GetComponentbyClass _unitcharacter "/Script/VR12ForTheKing.StatusComponent"))
  (bind _characterstatus (Variables|/Script/VR12ForTheKing.StatusComponent|GetCharacterStatus _returnvalue_2))
  (bind _returnvalue_3 (* (.intelligence _characterstatus) 5.0))
  (bind _returnvalue_4 (* _returnvalue_3 _returnvalue))
  ;[1 1 1] Unit의 Strength계수에 기본스텟을 곲하고 거기에 기본데미지값(5)에 데미지가 항상같게 나오지않게 랜덤값을 곱해서 반환
  (Development|PrintString (Utilities|String|ToString(Float) _returnvalue_4) true true "(R=0.000000,G=0.660000,B=1.000000,A=1.000000)" 6e+01)
  (return _returnvalue_4))

(fn ActionArrayRandomMagic
  (|CallParentFunction)
  (Development|PrintString "Doing RandomMagic" true true "(R=0.000000,G=0.660000,B=1.000000,A=1.000000)" 6e+01)
  (bind _asmy_game_mode_base (Utilities|Casting|CastToMyGameModeBase (Game|GetGameMode)))
  (switch Utilities|FlowControl|Switch|SwitchonEFactionType (Variables|Default|GetFactionType)
    (:Player
      (bind _actiontarget (Variables|Default|GetActionTarget)
        (:then
          _)
        (:else)))
    (:Enemy
      (Variables|Default|SetActionTarget (.OutItem (Utilities|Array|Random (Variables|/Script/VR12ForTheKing.MyGameModeBase|GetCharacterArray _asmy_game_mode_base))))))
  (if (Utilities|Enum|NotEqual(Enum) (Variables|/Script/VR12ForTheKing.BattleComponent|GetFactionType (Variables|/Script/VR12ForTheKing.MyCharacter|GetBattleComponent _actiontarget)) (Variables|Default|GetFactionType))
    (CallFunction|MagicCommand (.OutItem (Utilities|Array|Random (Variables|Abilities|GetBlackMagicAbilities))))
    (return)
    (else
      (Development|PrintString "Can not Attack Your Faction")
      (return))))