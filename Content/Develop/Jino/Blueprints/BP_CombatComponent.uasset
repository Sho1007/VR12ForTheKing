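; Combat component for BP_UnitBase actors that runs each unit's turn in a timer-driven battle.
; An HST-scaled timer requests turns from BP_BattleGameMode; party units get a command HUD, others target random party members, with a dynamic camera.
; Attacks use AI movement and scale pulses as placeholder animation, applying melee damage or spawning a projectile, then return home and restart the timer.
; Base damage currently returns only a random factor, leaving the STR formula unconnected.
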(event Custom|AttackCommand
  ;[1 1 1] 카메라가 유닛을따라다니도록
  (Class|BPDynamicCameraIT|SetOrbit(Message) (Pawn|GetViewTarget (Game|GetPlayerController 0)) false)
  ;[1 1 1] 근거리 원거리 유닛타입에 따라 공격방식이 다름
  (if (Variables|UnitStats|GetIsRangedCharacter)
    (CallFunction|RangeAttack)
    (else
      (CallFunction|MeleeAttack))))

(event Custom|RangeAttack
  (bind _unitcharacter (Variables|Default|GetUnitCharacter))
  (bind _unitcharacter_2 (Variables|Default|GetUnitCharacter))
  (bind _battlepostion (Variables|Default|GetBattlePostion))
  (bind (_location _rotation _scale) (Math|Transform|BreakTransform _battlepostion))
  ;[1 1 1] 근접공격 - 적에게 접근해서 공격해니메이션 실행하고 원래자리에 돌아온다. 공격이 끝나면 유닛의 턴이 끝나고 다음턴으로 이어짐
  (AI|AIMoveTo (Variables|Default|GetUnitCharacter) (CallFunction|GetRangePosition) 0 1e+02 false
    (:then
      (bind _actioncommandwindow (Variables|Default|GetActionCommandWindow)
        (:then
          (Widget|RemovefromParent _actioncommandwindow))
        (:else)))
    (:OnSuccess
      ;;[1 1 1] 원래는 AnimMontage를 통해서 애니메이션을 실행해야하나 스켈레탈매쉬가 없는 관계로 Printstring과 크기의 변화를 통해 공격표시
      (Development|PrintString (Utilities|String|Append (Utilities|String|ToString(Text) (Variables|/Game/Develop/Jino/Blueprints/BP_UnitBase.BP_UnitBase_C|GetName (Variables|Default|GetUnitCharacter))) "Attack->" (Utilities|String|ToString(Text) (Variables|/Game/Develop/Jino/Blueprints/BP_UnitBase.BP_UnitBase_C|GetName (Variables|Default|GetUnitTarget)))))
      (Transformation|SetActorScale3D _unitcharacter (* _scale 1.2))
      (Utilities|FlowControl|Delay 0.5)
      (Transformation|SetActorScale3D _unitcharacter _scale)
      (bind _returnvalue (Game|SpawnActorfromClass (Variables|Default|GetProjectileClass) (Transformation|GetActorTransform _unitcharacter_2) "Undefined" 0 _unitcharacter_2))
      (Game|BindEventtoOnEndPlay _returnvalue (delegate Custom|EndRangedAttack)))))

(event Custom|MeleeAttack
  (bind _battlepostion (Variables|Default|GetBattlePostion))
  (bind _unitcharacter (Variables|Default|GetUnitCharacter))
  (bind (_location _rotation _scale) (Math|Transform|BreakTransform _battlepostion))
  ;[1 1 1] 근접공격 - 적에게 접근해서 공격해니메이션 실행하고 원래자리에 돌아온다. 공격이 끝나면 유닛의 턴이 끝나고 다음턴으로 이어짐
  (AI|AIMoveTo (Variables|Default|GetUnitCharacter) "0, 0, 0" (Variables|Default|GetUnitTarget) 1e+02 false
    (:then
      (Development|PrintString "bbbbb")
      (bind _actioncommandwindow (Variables|Default|GetActionCommandWindow)
        (:then
          (Widget|RemovefromParent _actioncommandwindow))
        (:else)))
    (:OnSuccess
      ;;[1 1 1] 원래는 AnimMontage를 통해서 애니메이션을 실행해야하나 스켈레탈매쉬가 없는 관계로 Printstring과 크기의 변화를 통해 공격표시
      (Development|PrintString (Utilities|String|Append (Utilities|String|ToString(Text) (Variables|/Game/Develop/Jino/Blueprints/BP_UnitBase.BP_UnitBase_C|GetName (Variables|Default|GetUnitCharacter))) "Attack->" (Utilities|String|ToString(Text) (Variables|/Game/Develop/Jino/Blueprints/BP_UnitBase.BP_UnitBase_C|GetName (Variables|Default|GetUnitTarget)))))
      (Transformation|SetActorScale3D _unitcharacter (* _scale 1.4))
      (Utilities|FlowControl|Delay 0.5)
      (Transformation|SetActorScale3D _unitcharacter _scale)
      ;;[1 1 1] Damage를 입히는 노드
      (bind _asbp_unit_base (Utilities|Casting|CastToBP_UnitBase (Components|GetOwner)))
      (bind _basedamage (CallFunction|CalculateDamage))
      (Game|Damage|ApplyDamage (Variables|BP_CombatComponent_C|GetUnitTarget (Variables|/Game/Develop/Jino/Blueprints/BP_UnitBase.BP_UnitBase_C|GetBP_CombatComponent _asbp_unit_base)) _basedamage 0 _asbp_unit_base (Variables|Default|GetDamage%20Type%20Class))
      ;;[1 1 1] 원래 위치로 돌아올때 유닛의 보는 방향도 처음과 같게 하기, 돌아온다음에는 턴 끝내기
      (AI|AIMoveTo (Variables|Default|GetUnitCharacter) _location 0 5.0 false
        (:OnSuccess
          (Transformation|SetActorRotation (Variables|Default|GetUnitCharacter) _rotation)
          (Utilities|FlowControl|Delay 2.0)
          (CallFunction|EndUnitTurn))))))

(event Custom|EndRangedAttack
  (params (Actor :type Actor%20Object%20Reference) (EndPlayReason :type EEndPlayReason%20Enum :default "Destroyed"))
  (bind _battlepostion (Variables|Default|GetBattlePostion))
  (bind (_location _rotation _scale) (Math|Transform|BreakTransform _battlepostion))
  ;[1 1 1] 근접공격 - 적에게 접근해서 공격해니메이션 실행하고 원래자리에 돌아온다. 공격이 끝나면 유닛의 턴이 끝나고 다음턴으로 이어짐
  ;;[1 1 1] 원래 위치로 돌아올때 유닛의 보는 방향도 처음과 같게 하기, 돌아온다음에는 턴 끝내기
  (AI|AIMoveTo (Variables|Default|GetUnitCharacter) _location 0 5.0 false
    (:OnSuccess
      (Transformation|SetActorRotation (Variables|Default|GetUnitCharacter) _rotation)
      (Utilities|FlowControl|Delay 2.0)
      (CallFunction|EndUnitTurn))))

(event EventBeginPlay
  ;[1 1 1] 게임이 시작됐을 때 유닛들을 해당 유닛스폰위치에 스폰
  (bind _asbp_unit_base (Utilities|Casting|CastToBP_UnitBase (Components|GetOwner)))
  (bind _output_get (Variables|Default|SetUnitCharacter _asbp_unit_base))
  (Variables|Default|SetBattlePostion (Transformation|GetActorTransform _output_get))
  (CallFunction|BegineBattle)
  ;[1 1 1] 레벨에 따른 유닛들의 스텟설정 이단계에서는 아직 레벨이 같다면 모든 유닛의 스텟이 똑같다
  (bind _returnvalue (Utilities|GetDataTableRow "/Game/Develop/Jino/Blueprints/Data/BaseStatTable.BaseStatTable" (Utilities|String|StringToName (Utilities|String|ToString(Integer) (Variables|UnitStats|GetUnitLevel))))
    (:then
      (Variables|UnitStats|SetBaseUnitStat _returnvalue))))

(fn StartUnitTurn
  ;[1 1 1] StartUnitTurn함수가 호출되면 UnitCharacter가 PartyUnitBase클래스의 자식클래스인지를 확인해라
  (Development|PrintString "aaaaaa")
  (if (Utilities|ClassIsChildOf (Utilities|GetClass (Variables|Default|GetUnitCharacter)) "/Game/Develop/Jino/Blueprints/BP_PartyUnitBase.BP_PartyUnitBase_C")
    ;[1 1 1] PartyUnit의 자식클래스 가 맞다면 unit character의 actioncommand widget을 화면에 추가하고 set camera함수 호출
    (bind _returnvalue (UserInterface|CreateWidget "/Game/Develop/Jino/Blueprints/Widgets/BP_UnitBattleHud.BP_UnitBattleHud_C" 0 (Variables|Default|GetUnitCharacter)))
    (bind _output_get (Variables|Default|SetActionCommandWindow _returnvalue))
    (UserInterface|Viewport|AddtoViewport _output_get 0)
    (CallFunction|SetCamera)
    (else
      (bind _outactors (Actor|GetAllActorsOfClass "/Game/Develop/Jino/Blueprints/BP_PartyUnitBase.BP_PartyUnitBase_C"))
      (Variables|Default|SetUnitTarget (.OutItem (Utilities|Array|Random _outactors)))
      (switch int 0
        (:0
          (CallFunction|AttackCommand)
          (CallFunction|SetCamera))))))

(fn BegineBattle
  ;[1 1 1] 턴을 분배하는 공식 속도가 빠를수록 먼저 턴이 돌아온다.
  (bind _returnvalue (Utilities|Time|SetTimerbyFunctionName self "RequestTurn" (+ (* (- 1.0 (Math|Float|NormalizetoRange (Math|Conversions|ToFloat(Integer) (Utilities|Struct|BreakStatTableStruct (Variables|UnitStats|GetBaseUnitStat))) 0.0 255.0)) (- (Variables|UnitStats|GetMaxActionTime) (Variables|UnitStats|GetMinActionTime))) (Variables|UnitStats|GetMinActionTime))))
  (Variables|Default|SetActionTimer _returnvalue))

(fn EndUnitTurn
  ;[1 1 1] 턴이 끝나으면 BegineBattle을 호출해서 다음유닛의 턴이 오게함
  (Default|CallTurnEnded)
  (CallFunction|BegineBattle))

(fn RequestTurn
  (bind _asbp_battle_game_mode (Utilities|Casting|CastToBP_BattleGameMode (Game|GetGameMode)))
  (Default|TurnRequest _asbp_battle_game_mode (Variables|Default|GetUnitCharacter)))

(fn SetCamera
  (bind _returnvalue (Actor|GetActorOfClass "/Game/Develop/Jino/Blueprints/Cameras/BP_DynamicCamera.BP_DynamicCamera_C"))
  (Game|Player|SetViewTargetwithBlend (Game|GetPlayerController 0) _returnvalue 0.0 "VTBlend_Linear" 0.0 false)
  (Class|BPDynamicCameraIT|SetDynamicLocation(Message) _returnvalue (Variables|Default|GetUnitCharacter) "0, 0, 0")
  (Development|PrintString "Hello")
  (Class|BPDynamicCameraIT|SetOrbit(Message) (Pawn|GetViewTarget (Game|GetPlayerController 0)) true))

(fn CalculateDamage
  (bind _calculateddamage (CallFunction|CalculateBaseDamage))
  (return _calculateddamage))

(fn GetRangePosition
  (bind _unitcharacter (Variables|Default|GetUnitCharacter))
  (bind _returnvalue (Transformation|GetActorLocation _unitcharacter))
  (return (+ _returnvalue (* (Math|Vector|GetUnitDirection(Vector) _returnvalue (Transformation|GetActorLocation (Variables|Default|GetUnitTarget))) 5e+02))))

(fn CalculateBaseDamage
  ;[1 1 1] Unit의 Strength계수에 기본스텟을 곲하고 거기에 기본데미지값(5)에 데미지가 항상같게 나오지않게 랜덤값을 곱해서 반환
  (return (Math|Random|RandomFloatinRange 0.9 1.1)))

(fn CalculateDamageResistance
  (params (BaseDamage :type Float%20%28double-precision%29))
  ;[1 1 1] 들어온데미지를 제곱한것에 저항값으로 나눠서 캐릭터마다 다른 데미지가 들어오게
  (return (/ (Math|Float|Power BaseDamage 2.0) (+ BaseDamage (* (Utilities|Struct|BreakStatTableStruct (Variables|UnitStats|GetBaseUnitStat)) (Utilities|Struct|BreakStatModifier (Variables|UnitStats|GetUnitStatModifier)))))))